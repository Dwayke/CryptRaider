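; BP_Torch_Child is a child torch Blueprint that flickers its point light.
; Tick calls the parent, then enters a looping Delay of FlickerDelay that runs FlickerLight after each wait.
; FlickerLight picks a random intensity between the current value minus FlickerRange and the current value.
; Because each pick builds on the last, intensity only holds or drops, assuming a positive range and no external reset.
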(event EventBeginPlay
  (|CallParentFunction) ; This node is disabled and will not be called.\nDrag off pins to build functionality.
)

(event Collision|EventActorBeginOverlap
  (params (OtherActor :type Actor%20Object%20Reference))
  (|CallParentFunction OtherActor) ; This node is disabled and will not be called.\nDrag off pins to build functionality.
)

(event EventTick
  (params (DeltaSeconds :type Float%20%28single-precision%29))
  (|CallParentFunction DeltaSeconds)
  (Utilities|FlowControl|Delay (Variables|Default|GetFlickerDelay) :!label _label)
  (CallFunction|FlickerLight)
  (goto _label))

(fn ConstructionScript
  (|CallParentFunction))

(fn FlickerLight
  (bind _torch_pointlight (Variables|Default|GetTorch_PointLight))
  (bind _intensity (Variables|/Script/Engine.LightComponentBase|GetIntensity _torch_pointlight))
  (Rendering|Components|Light|SetIntensity (Variables|Default|GetTorch_PointLight) (Math|Random|RandomFloatinRange (- _intensity (Variables|Default|GetFlickerRange)) _intensity)))